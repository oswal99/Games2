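; Damage system component that tracks health, death, blocking and invincibility for its owner.
; TakeDamage uses a CanBeDamaged macro to route each damage info struct to blocked, applied or ignored, honoring its invincibility-bypass and blockable flags.
; Event dispatchers report blocks with parry eligibility, death, and damage responses when interruptible or forced.
; Heal, skipped once dead, sets Health to Amount minus current Health, clamped to MaxHealth, rather than adding.
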(fn `Heal`
  (params (Amount :type "Float (double-precision)"))
  (returns (NewHealth :type "Float (double-precision)"))
  (if (not (`self.Isdead`))
    (bind _output_get (set `self.Health` (`KismetMathLibrary.FClamp` (- Amount (`self.Health`)) 0.0 (`self.MaxHealth`))))
    (return _output_get)))

(fn `TakeDamage`
  (params (Damageinfo :type "/Game/MC-Archer/Damage/s_Damage Structure"))
  (returns (WasDamaged :type Boolean))
  (bind (_amount _damagetype _damageresponse _shoulddamageinvicible _canbeblock _canbeparried _shouldfir) (break `/Game/MC-Archer/Damage/s_Damage` Damageinfo))
  (`self.CanBeDamaged` _shoulddamageinvicible _canbeblock
    (:`BlockedDamage`
      (`self.OnBlocked` _canbeparried)
      (return false))
    (:`DoDamage`
      (bind _output_get (set `self.Health` (- (`self.Health`) _amount)))
      (if (<= _output_get 0.0)
        (set `self.Isdead` true)
        (`self.OnDeath`)
        (return true)
        (elif (or (`self.IsInterruptible`) _shouldfir)
          (`self.OnDamageResponse` _damageresponse)
          (return true))))
    (:`NoDamage`
      (return false))))